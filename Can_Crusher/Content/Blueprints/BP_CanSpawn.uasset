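; BP_CanSpawn is a can spawner actor for what appears to be a can-crusher game.
; On BeginPlay it starts a randomly timed looping timer and calls SpawnCan.
; SpawnCan gets a can from BP_Can_CrusherGamemode, activates its root and teleports it to relative zero, then sets a timer and calls DespawnCan.
; DespawnCan, also triggered by overlapping BP_DespawnZone, is empty, and the cached starting transform is unused.
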(event `self.ReceiveBeginPlay`
  (`self.Spawning Timer`))

(event `self.ReceiveActorBeginOverlap`
  (params (OtherActor :type "Actor Object Reference"))
  (if (== OtherActor "/Game/Blueprints/BP_DespawnZone.BP_DespawnZone")
    (`self.Despawn Can`)))

(fn `Despawn Can`)

(fn `Spawn Can`
  (`|ExecutionSequence`
    (:`then_0`
      (bind _asbp_can_crusher_gamemode (cast `/Game/Blueprints/BP_Can_CrusherGamemode` (`GameplayStatics.GetGameMode`)))
      (bind _currcan (`/Game/Blueprints/BP_Can_CrusherGamemode.GetCan` _asbp_can_crusher_gamemode))
      (`|ExecutionSequence`
        (:`then_0`
          (bind _rootcomponent (`Actor.RootComponent` _currcan))
          (`ActorComponent.Activate` _rootcomponent false))
        (:`then_1`
          (`SceneComponent.K2_SetRelativeLocation` _rootcomponent (0.0 0.0 0.0) false true))))
    (:`then_1`
      (`KismetSystemLibrary.K2_SetTimerDelegate` (`|CreateDelegate` :!event `Spawn Can`) 5.0)
      (`self.Despawn Can`))))

(fn `Spawning Timer`
  (`KismetSystemLibrary.K2_SetTimerDelegate` (`|CreateDelegate` :!event `Spawning Timer`) (`KismetMathLibrary.RandomFloatInRange` 0.001 3.5) true)
  (`self.Spawn Can`))

(fn `UserConstructionScript`
  (set `self.StartingLocation` (`self.GetTransform`)))