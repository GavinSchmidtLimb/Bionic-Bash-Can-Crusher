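; BP_Can_CrusherGamemode is the game mode for a can crusher game, handing out pooled cans per player.
; GetCan uses the player number to pick one of four object pools and stores the can at that pool's current index in CurrCan.
; It then increments that index, resetting it when it exceeds PoolSize; only this overflow branch is wired to return the can.
; BeginPlay initializes only the first pool's index.
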(event `self.ReceiveBeginPlay`
  (set `self.CurrIndex1` 0))

(fn `GetCan`
  (params (Player :type Integer))
  (returns (CurrCan :type "/Game/Blueprints/BP_Can Object Reference"))
  (bind _currindex1 (`self.CurrIndex1`))
  (bind _poolsize (`self.PoolSize`))
  (bind _currindex2 (`self.CurrIndex2`))
  (bind _currindex3 (`self.CurrIndex3`))
  (bind _currindex4 (`self.CurrIndex4`))
  ;[1 1 1] Set CurrCan according to player called
  (switch `int` Player
    (:`0`
      (set `self.CurrCan` (`|GetArrayItem` (`self.ObjectPool1`) _currindex1))
      ;[1 1 1] Keep index from overflow
      (bind _result (`/Engine/EditorBlueprintResources/StandardMacros.IncrementInt` _currindex1)
        (:`  `
          (`/Engine/EditorBlueprintResources/StandardMacros.CompareInt` _result _poolsize
            (:`>`
              (set `self.CurrIndex1` 0))))))
    (:`1`
      (set `self.CurrCan` (`|GetArrayItem` (`self.ObjectPool2`) _currindex2))
      (bind _result_2 (`/Engine/EditorBlueprintResources/StandardMacros.IncrementInt` _currindex2)
        (:`  `
          (`/Engine/EditorBlueprintResources/StandardMacros.CompareInt` _result_2 _poolsize
            (:`>`
              (set `self.CurrIndex2` 0))))))
    (:`2`
      (set `self.CurrCan` (`|GetArrayItem` (`self.ObjectPool3`) _currindex3))
      (bind _result_3 (`/Engine/EditorBlueprintResources/StandardMacros.IncrementInt` _currindex3)
        (:`  `
          (`/Engine/EditorBlueprintResources/StandardMacros.CompareInt` _result_3 _poolsize
            (:`>`
              (set `self.CurrIndex3` 0))))))
    (:`3`
      (set `self.CurrCan` (`|GetArrayItem` (`self.ObjectPool4`) _currindex4))
      (bind _result_4 (`/Engine/EditorBlueprintResources/StandardMacros.IncrementInt` _currindex4)
        (:`  `
          (`/Engine/EditorBlueprintResources/StandardMacros.CompareInt` _result_4 _poolsize
            (:`>`
              (set `self.CurrIndex4` 0)))))))
  (return (`self.CurrCan`)))

(fn `UserConstructionScript`
  (`parent.UserConstructionScript`))