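; BP_Can is a pooled can actor with a physics-driven cylinder, returned to its pool when it overlaps an actor tagged Despawn.
; Its SetinUse override calls the parent, toggles the cylinder's physics and gravity with the in-use state, then teleports it to the root's X and Y at a fixed height.
; OnReset destroys the actor outright instead of pooling it.
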(event `self.ReceiveActorBeginOverlap`
  (params (OtherActor :type "Actor Object Reference"))
  ;[1 1 1] Destroy on collision
  (if (`self.ActorHasTag` OtherActor "Despawn")
    (`self.ReturnToPool`)))

(event `self.SetInUse`
  (params (InUse :type Boolean))
  (bind _cylinder (`self.Cylinder`))
  (bind (_returnvalue_x _returnvalue_y) (`KismetMathLibrary.BreakVector` (`SceneComponent.K2_GetComponentLocation` (`self.DefaultSceneRoot`))))
  ;[1 1 1] Put Cylinder in correct spot
  (`parent.SetInUse` InUse)
  (`PrimitiveComponent.SetSimulatePhysics` _cylinder InUse)
  (`PrimitiveComponent.SetEnableGravity` _cylinder InUse)
  (`SceneComponent.K2_SetWorldLocation` (`self.Cylinder`) (`KismetMathLibrary.MakeVector` _returnvalue_x _returnvalue_y 800.0) false true))

(event `self.K2_OnReset`
  (`self.K2_DestroyActor`))

(fn `UserConstructionScript`
  (`parent.UserConstructionScript`))