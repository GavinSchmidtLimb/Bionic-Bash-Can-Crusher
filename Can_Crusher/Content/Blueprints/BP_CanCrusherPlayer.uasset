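; Player actor for a can-crushing minigame, where a hand catches falling cans to score points for its player number.
; Strong flex input or Space toggles the hand's crush collision, while analog flex and button inputs drive the Control Rig's hand closing.
; A randomized, self-restarting timer spawns pooled cans above a box, shrinking its maximum interval each spawn.
; Cans overlapping the active collision return to the pool and add a point.
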(event `StartSpawnTimer`
  ;[1 1 1] Begins timer for next spawn
  (`KismetSystemLibrary.K2_SetTimer` null "SpawnCans" (`KismetMathLibrary.RandomFloatInRange` (`self.MinSpawnInterval`) (`self.MaxSpawnInterval`))))

(event `self.K2_OnReset`
  ;[1 1 1] Cleanup from former session
  (`/Game/ObjectPool/BP_CanPool.CleanPool` (`self.BP_CanPool`))
  (`BasePointCounter.SetPoints` (`self.Base Point Counter`) (`self.PlayerNumber`) 0))

(event `Key|SpaceBar`
  (params (Key :type "Key Structure"))
  ;[1 1 1] Hand Controls
  (:`Pressed`
    (`self.CrushHand` :!label _label))
  (:`Released`
    (`self.OpenHand` :!label _label_2)))

(event `self.ReceiveBeginPlay`
  ;[1 1 1] Hand Controls
  (`self.OpenHand`)
  (`self.StartSpawnTimer`)
  (bind _asbp_can_crusher_gamemode (cast `/Game/Blueprints/BP_CanCrusherGamemode` (`GameplayStatics.GetGameMode`)))
  (set `self.Base Point Counter` (`/Game/Blueprints/BP_CanCrusherGamemode.BasePointCounter` _asbp_can_crusher_gamemode))
  (bind _astoon_hand_ctrl_rig (cast `` (`ControlRigComponent.GetControlRig`)))
  (set `self.HandRig` _astoon_hand_ctrl_rig)
  (`SceneComponent.SetMobility` "Static"))

(event `EnhancedInput|/LimbitlessBluetoothPlugin/InputActions/IA_StrongFlex`
  (params (ActionValue :type Boolean) (ElapsedSeconds :type "Float (double-precision)") (TriggeredSeconds :type "Float (double-precision)") (InputAction :type "InputAction Object Reference" :default "/LimbitlessBluetoothPlugin/InputActions/IA_StrongFlex.IA_StrongFlex"))
  ;[1 1 1] Hand Controls
  (:`Triggered`
    (goto _label))
  (:`Canceled`
    (goto _label_2)))

(event `EnhancedInput|/LimbitlessBluetoothPlugin/InputActions/IA_AnalogFlex`
  (params (ActionValue :type "Float (double-precision)") (ElapsedSeconds :type "Float (double-precision)") (TriggeredSeconds :type "Float (double-precision)") (InputAction :type "InputAction Object Reference" :default "/LimbitlessBluetoothPlugin/InputActions/IA_AnalogFlex.IA_AnalogFlex"))
  (bind _returnvalue (`|GetInputActionValue`))
  ;[1 1 1] Hand Controls
  (:`Triggered`
    (`/Engine/EditorBlueprintResources/StandardMacros.CompareFloat` _returnvalue :!label _label_3
      (:`>`
        _)
      (:`==`
        _))
    (set `self.FlexFloat` _returnvalue))
  (:`Started`
    (goto _label_3))
  (:`Ongoing`
    (goto _label_3))
  (:`Canceled`
    (goto _label_3))
  (:`Completed`
    (goto _label_3)))

(event `CrushHand`
  ;[1 1 1] Hand Controls
  (`PrimitiveComponent.SetCollisionEnabled` (`self.HandCrush`) "QueryAndPhysics"))

(event `OpenHand`
  ;[1 1 1] Hand Controls
  (`PrimitiveComponent.SetCollisionEnabled` (`self.HandCrush`) "NoCollision"))

(event `self.ReceiveTick`
  (params (DeltaSeconds :type "Float (single-precision)"))
  ;[1 1 1] Hand Controls
  (set `/Game/Blueprints/BP_CanCrusherPlayer.CloseAmount` (`self.FlexFloat`) (`self.HandRig`))
  (if (`|GetInputActionValue`)
    (set `self.FlexFloat` 1.0)
    (if (`|GetInputActionValue`)
      (set `self.FlexFloat` 1.0)
      (if (`|GetInputActionValue`)
        (set `self.FlexFloat` 1.0)))))

(event `self.HandCrush.OnComponentBeginOverlap`
  (params (OverlappedComponent :type "PrimitiveComponent Object Reference") (OtherActor :type "Actor Object Reference") (OtherComp :type "PrimitiveComponent Object Reference") (OtherBodyIndex :type Integer) (bFromSweep :type Boolean) (SweepResult :type "HitResult Structure (by ref)"))
  (bind _playernumber (`self.PlayerNumber`))
  (bind _base_point_counter (`self.Base Point Counter`))
  ;[1 1 1] Can Catching
  (bind _asbp_can (cast `/Game/ObjectPool/BP_Can` OtherActor))
  (`/Game/ObjectPool/BP_PooledCan.ReturnToPool` _asbp_can)
  (`BasePointCounter.AddPoints` _base_point_counter _playernumber 1)
  (`KismetSystemLibrary.PrintString` (`KismetStringLibrary.Conv_IntToString` (`BasePointCounter.GetPointsByPlayer` _base_point_counter _playernumber))))

(fn `AddPointToPlayer`
  (params (Amount :type Integer) (PlayerIndex :type Integer))
  (`self.AddPointToPlayer` Amount PlayerIndex))

(fn `SpawnCans`
  (bind _returnvalue (- (`self.MaxSpawnInterval`) 0.1))
  ;[1 1 1] Random Spawn in Box
  (bind _output_get (set `self.SpawnOrigin` (`SceneComponent.K2_GetComponentLocation` (`self.SpawnBox`))))
  (bind _output_get_2 (set `self.BoxExtent` (`BoxComponent.GetScaledBoxExtent` (`self.SpawnBox`))))
  (bind _output_get_3 (set `self.RandomX` (`KismetMathLibrary.RandomFloatInRange` (- (.x _output_get) (.x _output_get_2)) (+ (.x _output_get_2) (.x _output_get)))))
  (bind _output_get_4 (set `self.RandomY` (`KismetMathLibrary.RandomFloatInRange` (- (.y _output_get) (.y _output_get_2)) (+ (.y _output_get_2) (.y _output_get)))))
  (bind _output_get_5 (set `self.RandomZ` (`KismetMathLibrary.RandomFloatInRange` (+ (.z _output_get) 500.0) (+ (.z _output_get_2) (.z _output_get) 500.0))))
  (`/Game/ObjectPool/BP_CanPool.SpawnFromPool` (`self.BP_CanPool`) (`KismetMathLibrary.MakeTransform` (`KismetMathLibrary.MakeVector` _output_get_3 _output_get_4 _output_get_5)))
  ;[1 1 1] Check For Overflow
  (`/Engine/EditorBlueprintResources/StandardMacros.CompareFloat` _returnvalue
    (:`>`
      (set `self.MaxSpawnInterval` _returnvalue))
    (:`==`
      _)
    (:`<`
      _))
  (`self.StartSpawnTimer`))

(fn `UserConstructionScript`)