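; BP_CanPool is an object pool that pre-spawns can actors and hands them out for reuse.
; On BeginPlay it spawns instances of PooledCanClass in a loop up to PoolSize, storing each as not in use.
; SpawnFromPool takes the first free can, teleports it to the given transform and marks it in use, or prints a message when none is free.
; CleanPool destroys every pooled actor.
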(event `self.ReceiveBeginPlay`
  (`self.InitializePool`))

(event `InitializePool`
  (for _ (range (+ (`self.PoolSize`) 1))
    (bind _returnvalue (`|SpawnActorFromClass` (`self.PooledCanClass`) (`KismetMathLibrary.MakeTransform` (0.0 0.0 0.0)) "Undefined" "OverrideRootScale" null 10.0 null))
    (`KismetArrayLibrary.Array_AddUnique` (`self.CanPool`) _returnvalue)
    (`/Game/ObjectPool/BP_PooledCan.SetInUse` _returnvalue false)))

(fn `CleanPool`
  (for _array_element (`self.CanPool`)
    (`Actor.K2_DestroyActor` _array_element)))

(fn `FindFirstAvailableActor`
  (returns (PooledCan :type "/Game/ObjectPool/BP_PooledCan Object Reference"))
  (for _array_element (`self.CanPool`)
    (if (not (`/Game/ObjectPool/BP_PooledCan.InUse` _array_element))
      (return _array_element))))

(fn `SpawnFromPool`
  (params (SpawnTransform :type "Transform Structure"))
  (returns (PooledCan :type "/Game/ObjectPool/BP_PooledCan Object Reference"))
  (bind _pooledcan (`self.FindFirstAvailableActor`))
  (`/Engine/EditorBlueprintResources/StandardMacros.IsValid` _pooledcan
    (:`Is Valid`
      (`Actor.K2_SetActorTransform` _pooledcan SpawnTransform false true)
      (`/Game/ObjectPool/BP_PooledCan.SetInUse` _pooledcan true)
      (return _pooledcan))
    (:`Is Not Valid`
      (`KismetSystemLibrary.PrintString` "Could not find an can"))))