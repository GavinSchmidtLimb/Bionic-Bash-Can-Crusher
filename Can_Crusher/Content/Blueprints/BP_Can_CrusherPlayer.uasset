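; BP_Can_CrusherPlayer is a player Blueprint for a hand-crushing trigger, driven by the IA_LightFlex input.
; Triggering activates the ClosedHandCol collision component, then deactivates it after a short delay, or immediately on cancel.
; IsHandOpen is set opposite to its name, true while closing.
; BeginPlay disables mesh physics and deactivates the collider, whose overlap event only prints a debug message.
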(event `EnhancedInput|/LimbitlessBluetoothPlugin/InputActions/IA_LightFlex`
  (params (ActionValue :type Boolean) (ElapsedSeconds :type "Float (double-precision)") (TriggeredSeconds :type "Float (double-precision)") (InputAction :type "InputAction Object Reference" :default "/LimbitlessBluetoothPlugin/InputActions/IA_LightFlex.IA_LightFlex"))
  (bind _closedhandcol (`self.ClosedHandCol`))
  ;[1 1 1] Hand Crushing Trigger
  (:`Triggered`
    (`|ExecutionSequence`
      (:`then_0`
        (`KismetSystemLibrary.Delay` 0.5)
        (`ActorComponent.Deactivate` _closedhandcol :!label _label)
        (set `self.isHandOpen` false)
        (`KismetSystemLibrary.PrintString` "Opening"))
      (:`then_1`
        (`ActorComponent.Activate` _closedhandcol false)
        (set `self.isHandOpen` true)
        (`KismetSystemLibrary.PrintString` "Closing"))))
  (:`Canceled`
    (goto _label)))

(event `self.ReceiveBeginPlay`
  ;[1 1 1] Hand Crushing Trigger
  (`|ExecutionSequence`
    (:`then_0`
      (`PrimitiveComponent.SetSimulatePhysics` (`self.StaticMesh`) false))
    (:`then_1`
      (goto _label))))

(event `self.ClosedHandCol.OnComponentBeginOverlap`
  (params (OverlappedComponent :type "PrimitiveComponent Object Reference") (OtherActor :type "Actor Object Reference") (OtherComp :type "PrimitiveComponent Object Reference") (OtherBodyIndex :type Integer) (bFromSweep :type Boolean) (SweepResult :type "HitResult Structure (by ref)"))
  (`KismetSystemLibrary.PrintString` "Actor in hand"))

(fn `UserConstructionScript`)